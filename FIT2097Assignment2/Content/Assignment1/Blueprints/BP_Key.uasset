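; BP_Key is a collectible key pickup that hovers and spins in place.
; A Hover timeline started on BeginPlay sets the relative Z of both the key and its bounding box, while Tick rolls the key at a frame-rate-independent Rollspeed.
; When a FirstPersonCharacter overlaps the bounding box, it sets that character's HasKey flag and destroys itself.
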(event OnComponentBeginOverlap(BoundingBox)
  (params (OverlappedComponent :type Primitive%20Component%20Object%20Reference) (OtherActor :type Actor%20Object%20Reference) (OtherComp :type Primitive%20Component%20Object%20Reference) (OtherBodyIndex :type Integer) (bFromSweep :type Boolean) (SweepResult :type Hit%20Result%20Structure%20%28by%20ref%29))
  ;[1 1 1] Pick Up Key
  (bind _asfirst_person_character (Utilities|Casting|CastToFirstPersonCharacter OtherActor))
  (Variables|/Game/FirstPersonBP/Blueprints/FirstPersonCharacter.FirstPersonCharacter_C|SethasKey _asfirst_person_character true)
  (Actor|DestroyActor))

(event EventBeginPlay
  (bind _key (Variables|Default|GetKey))
  (bind _boundingbox (Variables|Default|GetBoundingBox))
  (bind _returnvalue (Transformation|GetRelativeTransform _key))
  (bind _returnvalue_2 (Transformation|GetRelativeTransform _boundingbox))
  ;[1 1 1] Makes the key hover
  (bind _hover (Timeline|Hover PlayFromStart)
    (:Update
      (Transformation|SetRelativeLocation (Variables|Default|GetKey) (Math|Vector|MakeVector (.x (.location _returnvalue)) (.y (.location _returnvalue)) _hover) false false)
      (Transformation|SetRelativeLocation (Variables|Default|GetBoundingBox) (Math|Vector|MakeVector (.x (.location _returnvalue_2)) (.y (.location _returnvalue_2)) _hover) false false))))

(event EventTick
  (params (DeltaSeconds :type Float%20%28single-precision%29))
  ;[1 1 1] Makes the key rotate in place
  (Transformation|AddRelativeRotation (Variables|Default|GetKey) (Math|Rotator|MakeRotator (* DeltaSeconds (Variables|Default|Getrollspeed)) 0.0 0.0) false false))

(fn ConstructionScript)