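; BP_BinaryCode is a three-switch binary code puzzle that unlocks a referenced Door.
; Overlapping a switch's box enables input, letting E flip that switch's state and emissive glow through a FlipFlop.
; Tick unlocks and lights the door only while A and C are on and flagged as needed and B is off, otherwise relocking it.
; B's check tests IsSwitchOnB twice, with no needed flag.
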(event OnComponentBeginOverlap(BoundingBoxA)
  (params (OverlappedComponent :type Primitive%20Component%20Object%20Reference) (OtherActor :type Actor%20Object%20Reference) (OtherComp :type Primitive%20Component%20Object%20Reference) (OtherBodyIndex :type Integer) (bFromSweep :type Boolean) (SweepResult :type Hit%20Result%20Structure%20%28by%20ref%29))
  ;[1 1 1] Toggles switchA
  (Input|EnableInput (Game|GetPlayerController 0))
  (Variables|Default|SetisOverlappingA true))

(event OnComponentEndOverlap(BoundingBoxA)
  (params (OverlappedComponent :type Primitive%20Component%20Object%20Reference) (OtherActor :type Actor%20Object%20Reference) (OtherComp :type Primitive%20Component%20Object%20Reference) (OtherBodyIndex :type Integer))
  ;[1 1 1] Toggles switchA
  (Input|DisableInput (Game|GetPlayerController 0))
  (Variables|Default|SetisOverlappingA false))

(event OnComponentBeginOverlap(BoundingBoxB)
  (params (OverlappedComponent :type Primitive%20Component%20Object%20Reference) (OtherActor :type Actor%20Object%20Reference) (OtherComp :type Primitive%20Component%20Object%20Reference) (OtherBodyIndex :type Integer) (bFromSweep :type Boolean) (SweepResult :type Hit%20Result%20Structure%20%28by%20ref%29))
  ;[1 1 1] Toggles switchB
  (Input|EnableInput (Game|GetPlayerController 0))
  (Variables|Default|SetisOverlappingB true))

(event OnComponentEndOverlap(BoundingBoxB)
  (params (OverlappedComponent :type Primitive%20Component%20Object%20Reference) (OtherActor :type Actor%20Object%20Reference) (OtherComp :type Primitive%20Component%20Object%20Reference) (OtherBodyIndex :type Integer))
  ;[1 1 1] Toggles switchB
  (Input|DisableInput (Game|GetPlayerController 0))
  (Variables|Default|SetisOverlappingB false))

(event OnComponentBeginOverlap(BoundingBoxC)
  (params (OverlappedComponent :type Primitive%20Component%20Object%20Reference) (OtherActor :type Actor%20Object%20Reference) (OtherComp :type Primitive%20Component%20Object%20Reference) (OtherBodyIndex :type Integer) (bFromSweep :type Boolean) (SweepResult :type Hit%20Result%20Structure%20%28by%20ref%29))
  ;[1 1 1] Toggles switchC
  (Input|EnableInput (Game|GetPlayerController 0))
  (Variables|Default|SetisOverlappingC true))

(event OnComponentEndOverlap(BoundingBoxC)
  (params (OverlappedComponent :type Primitive%20Component%20Object%20Reference) (OtherActor :type Actor%20Object%20Reference) (OtherComp :type Primitive%20Component%20Object%20Reference) (OtherBodyIndex :type Integer))
  ;[1 1 1] Toggles switchC
  (Input|DisableInput (Game|GetPlayerController 0))
  (Variables|Default|SetisOverlappingC false))

(event EventTick
  (params (DeltaSeconds :type Float%20%28single-precision%29))
  ;[1 1 1] Checks wether or not the correct code is pressed
  (if (Math|Boolean|ANDBoolean (and (Variables|Default|GetisSwitchNeededA) (Variables|Default|GetisSwitchOnA)) (not (and (Variables|Default|GetisSwitchOnB) (Variables|Default|GetisSwitchOnB))) (and (Variables|Default|GetisSwitchNeededC) (Variables|Default|GetIsSwitchOnC)))
    (Variables|/Game/Assignment1/Blueprints/BP_Door.BP_Door_C|SetisUnlocked (Variables|Default|GetDoor) true)
    (Utilities|FlowControl|DoOnce false
      (:Completed
        (Development|PrintString "The BinaryDoorCode is unlocked")
        (Rendering|Material|SetScalarParameterValueonMaterials (Variables|/Game/Assignment1/Blueprints/BP_Door.BP_Door_C|GetDoor (Variables|Default|GetDoor)) "BaseEmission" 1.0)))
    (else
      (Variables|/Game/Assignment1/Blueprints/BP_Door.BP_Door_C|SetisUnlocked (Variables|Default|GetDoor) false)
      (Rendering|Material|SetScalarParameterValueonMaterials (Variables|/Game/Assignment1/Blueprints/BP_Door.BP_Door_C|GetDoor (Variables|Default|GetDoor)) "BaseEmission" 0.0))))

(event Input|KeyboardEvents|E
  (params (Key :type Key%20Structure))
  ;[1 1 1] Toggles switchC
  (:Pressed
    (if (Variables|Default|GetisOverlappingC)
      (Utilities|FlowControl|FlipFlop
        (:A
          (Rendering|Material|SetScalarParameterValueonMaterials (Variables|Default|GetSwitchC) "BaseEmission" 1.0)
          (Variables|Default|SetIsSwitchOnC true))
        (:B
          (Rendering|Material|SetScalarParameterValueonMaterials (Variables|Default|GetSwitchC) "BaseEmission" 0.0)
          (Variables|Default|SetIsSwitchOnC false))))))

(event Input|KeyboardEvents|E
  (params (Key :type Key%20Structure))
  ;[1 1 1] Toggles switchB
  (:Pressed
    (if (Variables|Default|GetisOverlappingB)
      (Utilities|FlowControl|FlipFlop
        (:A
          (Rendering|Material|SetScalarParameterValueonMaterials (Variables|Default|GetSwitchB) "BaseEmission" 1.0)
          (Variables|Default|SetisSwitchOnB true))
        (:B
          (Rendering|Material|SetScalarParameterValueonMaterials (Variables|Default|GetSwitchB) "BaseEmission" 0.0)
          (Variables|Default|SetisSwitchOnB false))))))

(event Input|KeyboardEvents|E
  (params (Key :type Key%20Structure))
  ;[1 1 1] Toggles switchA
  (:Pressed
    (if (Variables|Default|GetisOverlappingA)
      (Utilities|FlowControl|FlipFlop
        (:A
          (Rendering|Material|SetScalarParameterValueonMaterials (Variables|Default|GetSwitchA) "BaseEmission" 1.0)
          (Variables|Default|SetisSwitchOnA true))
        (:B
          (Rendering|Material|SetScalarParameterValueonMaterials (Variables|Default|GetSwitchA) "BaseEmission" 0.0)
          (Variables|Default|SetisSwitchOnA false))))))

(fn ConstructionScript)