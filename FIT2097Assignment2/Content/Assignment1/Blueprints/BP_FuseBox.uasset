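; Fuse box actor that lets the player insert a carried fuse to unlock its referenced door.
; Overlapping the bounding box toggles input for the first player controller, so the E key works only nearby.
; On E, it casts the player to FirstPersonCharacter and checks HasFuse.
; If true, it reveals the fuse, sets the door's IsUnlocked, prints a message and raises the door material's BaseEmission.
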(event OnComponentBeginOverlap(BoundingBox)
  (params (OverlappedComponent :type Primitive%20Component%20Object%20Reference) (OtherActor :type Actor%20Object%20Reference) (OtherComp :type Primitive%20Component%20Object%20Reference) (OtherBodyIndex :type Integer) (bFromSweep :type Boolean) (SweepResult :type Hit%20Result%20Structure%20%28by%20ref%29))
  ;[1 1 1] Toggle input
  (Input|EnableInput (Game|GetPlayerController 0)))

(event OnComponentEndOverlap(BoundingBox)
  (params (OverlappedComponent :type Primitive%20Component%20Object%20Reference) (OtherActor :type Actor%20Object%20Reference) (OtherComp :type Primitive%20Component%20Object%20Reference) (OtherBodyIndex :type Integer))
  ;[1 1 1] Toggle input
  (Input|DisableInput (Game|GetPlayerController 0)))

(event Input|KeyboardEvents|E
  (params (Key :type Key%20Structure))
  (bind _door (Variables|Default|GetDoor))
  ;[1 1 1] Put fuse in when the player has a fuse
  (:Pressed
    (bind _asfirst_person_character (Utilities|Casting|CastToFirstPersonCharacter (Game|GetPlayerCharacter 0)))
    (if (Variables|/Game/FirstPersonBP/Blueprints/FirstPersonCharacter.FirstPersonCharacter_C|GethasFuse _asfirst_person_character)
      (Rendering|SetVisibility (Variables|Default|GetFuse) true false)
      (Variables|/Game/Assignment1/Blueprints/BP_Door.BP_Door_C|SetisUnlocked _door true)
      (Development|PrintString "The FuseDoor is unlocked")
      (Rendering|Material|SetScalarParameterValueonMaterials (Variables|/Game/Assignment1/Blueprints/BP_Door.BP_Door_C|GetDoor _door) "BaseEmission" 1.0))))

(fn ConstructionScript)