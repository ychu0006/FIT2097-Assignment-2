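; BP_Switch is a placeable switch that the player toggles with E to unlock or relock its linked doors.
; Overlapping its BoundingBox enables input, and leaving disables it.
; A FlipFlop alternates the on and off states, then loops the Doors array and sets IsUnlocked only on doors of the Switch Door type.
; The BaseEmission material parameter lights up the switch and those doors while on.
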(event OnComponentBeginOverlap(BoundingBox)
  (params (OverlappedComponent :type Primitive%20Component%20Object%20Reference) (OtherActor :type Actor%20Object%20Reference) (OtherComp :type Primitive%20Component%20Object%20Reference) (OtherBodyIndex :type Integer) (bFromSweep :type Boolean) (SweepResult :type Hit%20Result%20Structure%20%28by%20ref%29))
  ;[1 1 1] Toggles input
  (Input|EnableInput (Game|GetPlayerController 0)))

(event OnComponentEndOverlap(BoundingBox)
  (params (OverlappedComponent :type Primitive%20Component%20Object%20Reference) (OtherActor :type Actor%20Object%20Reference) (OtherComp :type Primitive%20Component%20Object%20Reference) (OtherBodyIndex :type Integer))
  ;[1 1 1] Toggles input
  (Input|DisableInput (Game|GetPlayerController 0)))

(event Input|KeyboardEvents|E
  (params (Key :type Key%20Structure))
  ;[1 1 1] Tgggles switch
  (:Pressed
    (Utilities|FlowControl|FlipFlop
      (:A
        (Variables|Default|SetisSwitchOn true)
        (Rendering|Material|SetScalarParameterValueonMaterials (Variables|Default|GetSwitch) "BaseEmission" 1.0)
        (for _array_element (Variables|Default|GetDoors)
          (switch Utilities|FlowControl|Switch|SwitchonE_DoorType (Variables|/Game/Assignment1/Blueprints/BP_Door.BP_Door_C|GetdoorType _array_element)
            (:NewEnumerator2
              (Variables|/Game/Assignment1/Blueprints/BP_Door.BP_Door_C|SetisUnlocked _array_element true)
              (Development|PrintString "A SwitchDoor is unlocked")
              (Rendering|Material|SetScalarParameterValueonMaterials (Variables|/Game/Assignment1/Blueprints/BP_Door.BP_Door_C|GetDoor _array_element) "BaseEmission" 1.0)))))
      (:B
        (Variables|Default|SetisSwitchOn false)
        (Rendering|Material|SetScalarParameterValueonMaterials (Variables|Default|GetSwitch) "BaseEmission" 0.0)
        (for _array_element_2 (Variables|Default|GetDoors)
          (switch Utilities|FlowControl|Switch|SwitchonE_DoorType (Variables|/Game/Assignment1/Blueprints/BP_Door.BP_Door_C|GetdoorType _array_element_2)
            (:NewEnumerator2
              (Variables|/Game/Assignment1/Blueprints/BP_Door.BP_Door_C|SetisUnlocked _array_element_2 false)
              (Rendering|Material|SetScalarParameterValueonMaterials (Variables|/Game/Assignment1/Blueprints/BP_Door.BP_Door_C|GetDoor _array_element_2) "BaseEmission" 0.0))))))))

(fn ConstructionScript)