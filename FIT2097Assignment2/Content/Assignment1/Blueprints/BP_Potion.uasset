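; BP_Potion is a health pickup that hovers and spins in the level.
; A Hover timeline started on BeginPlay drives the relative Z of both the Potion and its BoundingBox, while Tick yaws the potion at YawSpeed scaled by DeltaSeconds.
; When a FirstPersonCharacter overlaps the BoundingBox, its CurrentHealth is set to MaxHealth and the potion destroys itself.
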(event OnComponentBeginOverlap(BoundingBox)
  (params (OverlappedComponent :type Primitive%20Component%20Object%20Reference) (OtherActor :type Actor%20Object%20Reference) (OtherComp :type Primitive%20Component%20Object%20Reference) (OtherBodyIndex :type Integer) (bFromSweep :type Boolean) (SweepResult :type Hit%20Result%20Structure%20%28by%20ref%29))
  ;[1 1 1] Heal player
  (bind _asfirst_person_character (Utilities|Casting|CastToFirstPersonCharacter OtherActor))
  (Variables|/Game/FirstPersonBP/Blueprints/FirstPersonCharacter.FirstPersonCharacter_C|SetcurrentHealth _asfirst_person_character (Variables|/Game/FirstPersonBP/Blueprints/FirstPersonCharacter.FirstPersonCharacter_C|GetmaxHealth _asfirst_person_character))
  (Actor|DestroyActor))

(event EventBeginPlay
  (bind _potion (Variables|Default|GetPotion))
  (bind _boundingbox (Variables|Default|GetBoundingBox))
  (bind _returnvalue (Transformation|GetRelativeTransform _potion))
  (bind _returnvalue_2 (Transformation|GetRelativeTransform _boundingbox))
  ;[1 1 1] Make potion hover
  (bind _hover (Timeline|Hover Play)
    (:Update
      (Transformation|SetRelativeLocation (Variables|Default|GetPotion) (Math|Vector|MakeVector (.x (.location _returnvalue)) (.y (.location _returnvalue)) _hover) false false)
      (Transformation|SetRelativeLocation (Variables|Default|GetBoundingBox) (Math|Vector|MakeVector (.x (.location _returnvalue_2)) (.y (.location _returnvalue_2)) _hover) false false))))

(event EventTick
  (params (DeltaSeconds :type Float%20%28single-precision%29))
  ;[1 1 1] Make potion rotate
  (Transformation|AddRelativeRotation (Variables|Default|GetPotion) (Math|Rotator|MakeRotator 0.0 0.0 (* DeltaSeconds (Variables|Default|GetyawSpeed))) false false))

(fn ConstructionScript)