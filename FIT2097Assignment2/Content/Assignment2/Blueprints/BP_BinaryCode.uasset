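; Binary code puzzle that unlocks a referenced Door when its switches form the required combination.
; Tick requires A and C both needed and on and B off, ignoring any needed flag for B.
; FlipFlops toggle switch state and emissive glow: A via WasToggled, C via E, while B's logic is unconnected.
; Unlock message and door glow sit behind an unreset DoOnce, so the glow never returns after relocking.
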(event EventWasToggled
  ;[1 1 1] Toggles switchA
  (if true
    (Utilities|FlowControl|FlipFlop
      (:A
        (Rendering|Material|SetScalarParameterValueonMaterials (Variables|Default|GetSwitchA) "BaseEmission" 1.0)
        (Variables|Default|SetisSwitchOnA true))
      (:B
        (Rendering|Material|SetScalarParameterValueonMaterials (Variables|Default|GetSwitchA) "BaseEmission" 0.0)
        (Variables|Default|SetisSwitchOnA false)))))

(event EventTick
  (params (DeltaSeconds :type Float%20%28single-precision%29))
  ;[1 1 1] Checks wether or not the correct code is pressed
  (if (Math|Boolean|ANDBoolean (and (Variables|Default|GetisSwitchNeededA) (Variables|Default|GetisSwitchOnA)) (not (and (Variables|Default|GetisSwitchOnB) (Variables|Default|GetisSwitchOnB))) (and (Variables|Default|GetisSwitchNeededC) (Variables|Default|GetIsSwitchOnC)))
    (Variables|/Game/Assignment2/Blueprints/BP_Door.BP_Door_C|SetisUnlocked (Variables|Default|GetDoor) true)
    (Utilities|FlowControl|DoOnce false
      (:Completed
        (Development|PrintString "The BinaryDoorCode is unlocked")
        (Rendering|Material|SetScalarParameterValueonMaterials (Variables|/Game/Assignment2/Blueprints/BP_Door.BP_Door_C|GetDoor (Variables|Default|GetDoor)) "BaseEmission" 1.0)))
    (else
      (Variables|/Game/Assignment2/Blueprints/BP_Door.BP_Door_C|SetisUnlocked (Variables|Default|GetDoor) false)
      (Rendering|Material|SetScalarParameterValueonMaterials (Variables|/Game/Assignment2/Blueprints/BP_Door.BP_Door_C|GetDoor (Variables|Default|GetDoor)) "BaseEmission" 0.0))))

(event Input|KeyboardEvents|E
  (params (Key :type Key%20Structure))
  ;[1 1 1] Toggles switchC
  (:Pressed
    (if true
      (Utilities|FlowControl|FlipFlop
        (:A
          (Rendering|Material|SetScalarParameterValueonMaterials (Variables|Default|GetSwitchC) "BaseEmission" 1.0)
          (Variables|Default|SetIsSwitchOnC true))
        (:B
          (Rendering|Material|SetScalarParameterValueonMaterials (Variables|Default|GetSwitchC) "BaseEmission" 0.0)
          (Variables|Default|SetIsSwitchOnC false))))))

(fn ConstructionScript)