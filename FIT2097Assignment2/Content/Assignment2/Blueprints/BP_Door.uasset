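; BP_Door is an interactive door with five types: default, key, switch, fuse and binary code.
; The construction script picks materials by type and locks all but default doors, using emission to mark unlocked ones.
; Overlapping its box enables input, letting E toggle a timeline swing through a FlipFlop when unlocked.
; Key doors unlock themselves if the player has a key; other locked types have no unlock logic here.
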(event OnComponentBeginOverlap(BoundingBox)
  (params (OverlappedComponent :type Primitive%20Component%20Object%20Reference) (OtherActor :type Actor%20Object%20Reference) (OtherComp :type Primitive%20Component%20Object%20Reference) (OtherBodyIndex :type Integer) (bFromSweep :type Boolean) (SweepResult :type Hit%20Result%20Structure%20%28by%20ref%29))
  ;[1 1 1] Toggle input
  (Input|EnableInput (Game|GetPlayerController 0)))

(event OnComponentEndOverlap(BoundingBox)
  (params (OverlappedComponent :type Primitive%20Component%20Object%20Reference) (OtherActor :type Actor%20Object%20Reference) (OtherComp :type Primitive%20Component%20Object%20Reference) (OtherBodyIndex :type Integer))
  ;[1 1 1] Toggle input
  (Input|DisableInput (Game|GetPlayerController 0)))

(event Input|KeyboardEvents|E
  (params (Key :type Key%20Structure))
  ;[1 1 1] Check whether or not to open/close door based on door type and if it's unlocked
  (:Pressed
    (switch Utilities|FlowControl|Switch|SwitchonE_DoorType (Variables|Default|GetdoorType)
      (:NewEnumerator0
        (if (Variables|Default|GetisUnlocked) :!label _label
          (Utilities|FlowControl|FlipFlop :!label _label_2
            (:A
              (bind _rotation (Timeline|Door%20Open%20and%20Close PlayFromStart)
                (:Update
                  (Transformation|SetRelativeRotation (Variables|Default|GetDoor) (Math|Rotator|MakeRotator 0.0 0.0 _rotation) false false))))
            (:B
              (Timeline|Door%20Open%20and%20Close Reverse)))))
      (:NewEnumerator1
        (if (Variables|Default|GetisUnlocked)
          (goto _label_2)
          (else
            (bind _asfirst_person_character (Utilities|Casting|CastToFirstPersonCharacter (Game|GetPlayerCharacter 0)))
            (if (Variables|/Game/FirstPersonBP/Blueprints/FirstPersonCharacter.FirstPersonCharacter_C|GethasKey _asfirst_person_character)
              (Variables|Default|SetisUnlocked true)
              (Development|PrintString "The KeyDoor is unlocked")
              (Rendering|Material|SetScalarParameterValueonMaterials (Variables|Default|GetDoor) "BaseEmission" 1.0)
              (goto _label)))))
      (:NewEnumerator2
        (goto _label))
      (:NewEnumerator3
        (goto _label))
      (:NewEnumerator4
        (goto _label)))))

(fn ConstructionScript
  (Rendering|Material|SetMaterial (Variables|Default|GetDoor) 0 (Utilities|Select :Index (Variables|Default|GetdoorType) :NewEnumerator0 "/Game/Assignment1/Materials/M_Door.M_Door" :NewEnumerator1 "/Game/Assignment1/Materials/M_KeyDoor.M_KeyDoor" :NewEnumerator2 "/Game/Assignment1/Materials/M_SwitchDoor.M_SwitchDoor" :NewEnumerator3 "/Game/Assignment1/Materials/M_FuseDoor.M_FuseDoor" :NewEnumerator4 "/Game/Assignment1/Materials/M_BinaryDoorCode.M_BinaryDoorCode"))
  (Rendering|Material|SetMaterial (Variables|Default|GetDoor%20Frame) 0 (Utilities|Select :Index (Variables|Default|GetdoorType) :NewEnumerator0 "/Game/Assignment1/Materials/M_Door.M_Door" :NewEnumerator1 "/Game/Assignment1/Materials/M_KeyDoor.M_KeyDoor" :NewEnumerator2 "/Game/Assignment1/Materials/M_SwitchDoor.M_SwitchDoor" :NewEnumerator3 "/Game/Assignment1/Materials/M_FuseDoor.M_FuseDoor" :NewEnumerator4 "/Game/Assignment1/Materials/M_BinaryDoorCode.M_BinaryDoorCode"))
  (if (Utilities|Select :Index (Variables|Default|GetdoorType) :NewEnumerator0 false :NewEnumerator1 true :NewEnumerator2 true :NewEnumerator3 true :NewEnumerator4 true)
    (Variables|Default|SetisUnlocked false)
    (else
      (Variables|Default|SetisUnlocked true)
      (Rendering|Material|SetScalarParameterValueonMaterials (Variables|Default|GetDoor) "BaseEmission" 1.0))))