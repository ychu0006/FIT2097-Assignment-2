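; BP_Fuse is a collectible fuse pickup that hovers and spins in the level.
; A timeline started on BeginPlay drives the relative Z of the mesh and its bounding box together, while Tick rolls the mesh at RollSpeed.
; When a FirstPersonCharacter overlaps the bounding box, it sets that character's HasFuse flag and destroys itself.
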(event OnComponentBeginOverlap(BoundingBox)
  (params (OverlappedComponent :type Primitive%20Component%20Object%20Reference) (OtherActor :type Actor%20Object%20Reference) (OtherComp :type Primitive%20Component%20Object%20Reference) (OtherBodyIndex :type Integer) (bFromSweep :type Boolean) (SweepResult :type Hit%20Result%20Structure%20%28by%20ref%29))
  ;[1 1 1] Pick Up Fuse
  (bind _asfirst_person_character (Utilities|Casting|CastToFirstPersonCharacter OtherActor))
  (Variables|/Game/FirstPersonBP/Blueprints/FirstPersonCharacter.FirstPersonCharacter_C|SethasFuse _asfirst_person_character true)
  (Actor|DestroyActor))

(event EventBeginPlay
  (bind _fuse (Variables|Default|GetFuse))
  (bind _boundingbox (Variables|Default|GetBoundingBox))
  (bind _returnvalue (Transformation|GetRelativeTransform _fuse))
  (bind _returnvalue_2 (Transformation|GetRelativeTransform _boundingbox))
  ;[1 1 1] Makes the fuse hover
  (bind _hover (Timeline|Timeline_1 PlayFromStart)
    (:Update
      (Transformation|SetRelativeLocation (Variables|Default|GetFuse) (Math|Vector|MakeVector (.x (.location _returnvalue)) (.y (.location _returnvalue)) _hover) false false)
      (Transformation|SetRelativeLocation (Variables|Default|GetBoundingBox) (Math|Vector|MakeVector (.x (.location _returnvalue_2)) (.y (.location _returnvalue_2)) _hover) false false))))

(event EventTick
  (params (DeltaSeconds :type Float%20%28single-precision%29))
  ;[1 1 1] Makes the fuse rotate in place
  (Transformation|AddRelativeRotation (Variables|Default|GetFuse) (Math|Rotator|MakeRotator (* DeltaSeconds (Variables|Default|GetrollSpeed)) 0.0 0.0) false false))

(fn ConstructionScript)