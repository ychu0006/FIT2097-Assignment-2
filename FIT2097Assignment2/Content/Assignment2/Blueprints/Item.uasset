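; Item actor that represents a health potion, key or fuse in the level, selected by its ItemType.
; The construction script sets the static mesh, materials and scale to match the type.
; On BeginPlay the Hover timeline starts, adding its value to the mesh's relative Z each update as an offset rather than setting an absolute height.
; No pickup or interaction logic is present in these graphs.
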(event EventBeginPlay
  (bind _hover (Timeline|Hover Play)
    (:Update
      (Transformation|AddRelativeLocation (Variables|Default|GetStaticMesh) (Math|Vector|MakeVector 0.0 0.0 _hover) false false))))

(fn ConstructionScript
  (switch Utilities|FlowControl|Switch|SwitchonEItemType (Variables|Default|GetItemType)
    (:HEALTH
      (Components|StaticMesh|SetStaticMesh (Variables|Default|GetStaticMesh) "/Game/Assignment2/Materials/PotionA.PotionA")
      (Rendering|Material|SetMaterial (Variables|Default|GetStaticMesh) 0 "/Game/Assignment2/Materials/Liquid.Liquid")
      (Rendering|Material|SetMaterial (Variables|Default|GetStaticMesh) 1 "/Game/Assignment2/Materials/Glass.Glass")
      (Rendering|Material|SetMaterial (Variables|Default|GetStaticMesh) 2 "/Game/Assignment2/Materials/Cork.Cork")
      (Transformation|SetRelativeScale3D (Variables|Default|GetStaticMesh) "0.500000,0.500000,0.500000"))
    (:KEY
      (Components|StaticMesh|SetStaticMesh (Variables|Default|GetStaticMesh) "/Game/Assignment2/Materials/key.key")
      (Rendering|Material|SetMaterial (Variables|Default|GetStaticMesh) 0 "/Game/Assignment2/Materials/Metal_756_x_512_px_3109ALUMOX_Mat.Metal_756_x_512_px_3109ALUMOX_Mat")
      (Transformation|SetRelativeScale3D (Variables|Default|GetStaticMesh) "0.250000,0.250000,0.250000"))
    (:FUSE
      (Components|StaticMesh|SetStaticMesh (Variables|Default|GetStaticMesh) "/Game/StarterContent/Shapes/Shape_Cylinder.Shape_Cylinder")
      (Rendering|Material|SetMaterial (Variables|Default|GetStaticMesh) 0 "/Game/Assignment2/Materials/M_Fuse.M_Fuse")
      (Transformation|SetRelativeScale3D (Variables|Default|GetStaticMesh) "0.100000,0.050000,0.180000"))))